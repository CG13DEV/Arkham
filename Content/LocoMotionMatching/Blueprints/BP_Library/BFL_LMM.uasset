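; BFL_LMM is a Blueprint function library of math helpers for the LocoMotionMatching system.
; It derives velocity and squared XY speed from two timed position samples.
; Its fixed dynamic weighted moving average smooths rotators per axis, scaling the weight with angular distance from the previous sample.
; Angle helpers take the shortest path across the ±180 degree wrap and normalize results.
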(fn GetVelocityBetweenTwoSamples
  (params (Start :type Pose%20Search%20Query%20Trajectory%20Sample%20Structure%20%28by%20ref%29) (End :type Pose%20Search%20Query%20Trajectory%20Sample%20Structure%20%28by%20ref%29))
  (bind (_facing _position _accumulatedseconds) (Utilities|Struct|BreakPoseSearchQueryTrajectorySample End))
  (bind (_facing_2 _position_2 _accumulatedseconds_2) (Utilities|Struct|BreakPoseSearchQueryTrajectorySample Start))
  (bind _returnvalue (- _accumulatedseconds_2 _accumulatedseconds))
  (bind _returnvalue_2 (- _position _position_2))
  (bind _returnvalue_3 (/ _returnvalue_2 _returnvalue))
  (return _returnvalue_3 (Class|KismetMathLibrary|VSizeXYSquared _returnvalue_3)))

(fn DynamicWeightedMovingAverageRotator(Fixed)
  (params (Current%20Sample :type Rotator) (Previous%20Sample :type Rotator) (Max%20Distance :type Float%20%28double-precision%29) (Min%20Weight :type Float%20%28double-precision%29) (Max%20Weight :type Float%20%28double-precision%29))
  (bind ___worldcontext (LocalVariables|Get__WorldContext))
  (bind (_roll _pitch _yaw) (Math|Rotator|BreakRotator Previous%20Sample))
  (bind (_roll_2 _pitch_2 _yaw_2) (Math|Rotator|BreakRotator Current%20Sample))
  (return (Math|Rotator|MakeRotator (Rotation|DynamicWeightedMovingAverageAngle _roll_2 _roll Max%20Distance Min%20Weight Max%20Weight ___worldcontext) (Rotation|DynamicWeightedMovingAverageAngle _pitch_2 _pitch Max%20Distance Min%20Weight Max%20Weight ___worldcontext) (Rotation|DynamicWeightedMovingAverageAngle _yaw_2 _yaw Max%20Distance Min%20Weight Max%20Weight ___worldcontext))))

(fn AngleDistance
  (params (FromAngle :type Float%20%28double-precision%29) (ToAngle :type Float%20%28double-precision%29))
  (LocalVariables|SetDist (- (Math|Rotator|NormalizeAxis ToAngle) (Math|Rotator|NormalizeAxis FromAngle)))
  (if (>= (LocalVariables|GetDist) 1.8e+02)
    (return (- (LocalVariables|GetDist) 3.6e+02))
    (elif (< (LocalVariables|GetDist) -1.8e+02)
      (return (+ (LocalVariables|GetDist) 3.6e+02))
      (else
        (return (LocalVariables|GetDist))))))

(fn DynamicWeightedMovingAverageAngle
  (params (Current%20Sample :type Float%20%28double-precision%29) (Previous%20Sample :type Float%20%28double-precision%29) (Max%20Distance :type Float%20%28double-precision%29) (Min%20Weight :type Float%20%28double-precision%29) (Max%20Weight :type Float%20%28double-precision%29))
  (LocalVariables|SetDistance (Math|Float|Absolute(Float) (Rotation|AngleDistance Previous%20Sample Current%20Sample (LocalVariables|Get__WorldContext))))
  (LocalVariables|SetWeight Min%20Weight)
  (if (> Max%20Distance 0.0)
    (LocalVariables|SetWeight (Math|Float|Lerp Min%20Weight Max%20Weight (Math|Float|Clamp(Float) (/ (LocalVariables|GetDistance) Max%20Distance)))))
  (return (Rotation|WeightedMovingAverageAngle Current%20Sample Previous%20Sample (LocalVariables|GetWeight) (LocalVariables|Get__WorldContext))))

(fn WeightedMovingAverageAngle
  (params (Current%20Sample :type Float%20%28double-precision%29) (Previous%20Sample :type Float%20%28double-precision%29) (Weight :type Float%20%28double-precision%29))
  (return (Math|Rotator|NormalizeAxis (+ Previous%20Sample (* (Rotation|AngleDistance Previous%20Sample Current%20Sample (LocalVariables|Get__WorldContext)) (Math|Float|Clamp(Float) Weight))))))

(fn NormaliseAngle
  (params (Angle :type Float%20%28double-precision%29))
  (return (- (Math|Float|%(Float) (+ Angle 1.8e+02) 3.6e+02) 1.8e+02)))