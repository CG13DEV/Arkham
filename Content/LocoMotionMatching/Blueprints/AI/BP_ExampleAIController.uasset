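; Example AI controller for the LocoMotionMatching system that makes non-player pawns wander.
; Three seconds after possession, it focuses on the player pawn and starts a loop of moves to random reachable nearby points.
; The loop reissues on a fixed delay after each AIMoveTo call, without waiting for arrival.
; Helper functions, uncalled here, send random gait and rotation mode changes to the pawn through character messages.
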(event Custom|Move%20to%20Random%20Location
  (AI|AIMoveTo (Variables|Default|GetPossessed%20Pawn) (.RandomLocation (AI|Navigation|GetRandomReachablePointinRadius (Transformation|GetActorLocation (Variables|Default|GetPossessed%20Pawn)) 1e+03 0 0)) 0 5.0 false
    (:then
      (Utilities|FlowControl|Delay 1e+01)
      (CallFunction|MovetoRandomLocation))))

(event EventPossess
  (params (PossessedPawn :type Pawn%20Object%20Reference))
  (Variables|Default|SetPossessed%20Pawn PossessedPawn)
  (Utilities|FlowControl|Delay 3.0)
  (if (not (Pawn|IsPlayerControlled (Variables|Default|GetPossessed%20Pawn)))
    (AI|SetFocus (Game|Player|GetPlayerPawn 0))
    (CallFunction|MovetoRandomLocation)))

(fn ConstructionScript)

(fn InitRandomGait
  (Class|BPILMMCharacter|SetGait(Character)(Message) (Variables|Default|GetPossessed%20Pawn) (select (Math|Random|RandomBool) "NewEnumerator1" "NewEnumerator0")))

(fn UpdateRotationMode
  (params (New%20Rotation%20Mode :type LocomotionRotationMode%20Enum :default "NewEnumerator0"))
  (Class|BPILMMCharacter|SetRotationMode(Character)(Message) (Variables|Default|GetPossessed%20Pawn) New%20Rotation%20Mode))