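; Animation modifier that bakes FootLock_L and FootLock_R float curves marking when each foot is planted.
; Plants start at footstep notifies, less a margin, or at time zero if the foot starts low, and notifies get their type and side set.
; A frame-by-frame scan of foot and ball bone heights finds each lift, and keys are kept in time order.
; Revert removes notify tracks with the curve names, not the curves.
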(event EventOnApply
  (params (AnimationSequence :type Anim%20Sequence%20Object%20Reference))
  (Variables|Default|SetAnim%20Sequence AnimationSequence)
  (CallFunction|ProcessNotifies (Class|AnimationBlueprintLibrary|GetAnimationNotifyEventsforTrack (Variables|Default|GetAnim%20Sequence) "FootLock_L_Notifs") true)
  (CallFunction|ProcessNotifies (Class|AnimationBlueprintLibrary|GetAnimationNotifyEventsforTrack (Variables|Default|GetAnim%20Sequence) "FootLock_R_Notifs") false))

(event EventOnRevert
  (params (AnimationSequence :type Anim%20Sequence%20Object%20Reference))
  (Class|AnimationBlueprintLibrary|RemoveAnimationNotifyTrack AnimationSequence "FootLock_L")
  (Class|AnimationBlueprintLibrary|RemoveAnimationNotifyTrack AnimationSequence "FootLock_R"))

(fn ProcessNotifies
  (params (Notifies :type Array%20of%20Anim%20Notify%20Event%20Structures) (LeftFoot :type Boolean))
  (Variables|Default|SetEarliest%20Safe%20Time 0.0)
  (bind _new_curve (CallFunction|CreateCurve LeftFoot))
  (LocalVariables|SetCurve _new_curve)
  (for _array_element Notifies
    (LocalVariables|SetCurrentNotify _array_element)
    (CallFunction|AddKey (LocalVariables|GetCurve) (- (Class|AnimationBlueprintLibrary|GetAnimNotifyEventTriggerTime (LocalVariables|GetCurrentNotify)) (Variables|Default|GetFootstepStartMargin)) (Variables|Default|GetPlantHeightValue))
    (CallFunction|SetNotifyParams (Utilities|Struct|BreakAnimNotifyEvent (LocalVariables|GetCurrentNotify)) LeftFoot)
    (if (.FootLifted (CallFunction|GetFootstepEnd (Class|AnimationBlueprintLibrary|GetAnimNotifyEventTriggerTime (LocalVariables|GetCurrentNotify)) LeftFoot))
      (CallFunction|AddFootstepEndKeys (LocalVariables|GetCurve) (.EndTime (CallFunction|GetFootstepEnd (Class|AnimationBlueprintLibrary|GetAnimNotifyEventTriggerTime (LocalVariables|GetCurrentNotify)) LeftFoot))))))

(fn CreateCurve
  (params (Left%20Foot :type Boolean))
  (LocalVariables|SetFoot%20Bone (select Left%20Foot "foot_l" "foot_r"))
  (LocalVariables|SetBall%20Bone (select Left%20Foot "ball_l" "ball_r"))
  (LocalVariables|SetCurve%20Name (select Left%20Foot "FootLock_L" "FootLock_R"))
  (bind _returnvalue (Class|AnimationBlueprintLibrary|DoesCurveExist (Variables|Default|GetAnim%20Sequence) (LocalVariables|GetCurve%20Name) "RCT_Float"))
  (if _returnvalue
    (Class|AnimationBlueprintLibrary|RemoveCurve (Variables|Default|GetAnim%20Sequence) (LocalVariables|GetCurve%20Name) false))
  (Class|AnimationBlueprintLibrary|AddCurve (Variables|Default|GetAnim%20Sequence) (LocalVariables|GetCurve%20Name) "RCT_Float" false)
  (CallFunction|InitCurveKeys (LocalVariables|GetCurve%20Name) Left%20Foot)
  (return (LocalVariables|GetCurve%20Name)))

(fn GetFootstepEnd
  (params (StepStartTime :type Float%20%28double-precision%29) (IsLeft :type Boolean))
  (bind _anim_sequence (Variables|Default|GetAnim%20Sequence))
  (bind _anim_sequence_2 (Variables|Default|GetAnim%20Sequence))
  (LocalVariables|SetFootLiftFound false)
  (LocalVariables|SetFootBoneName (select IsLeft "foot_l" "foot_r"))
  (LocalVariables|SetBallBoneName (select IsLeft "ball_l" "ball_r"))
  (LocalVariables|SetStartFootHeight (Math|Float|Min(Float) (.z (.Location (CallFunction|GetBonePoseHelperTime _anim_sequence_2 (LocalVariables|GetFootBoneName) StepStartTime))) (.z (.Location (CallFunction|GetBonePoseHelperTime _anim_sequence_2 (LocalVariables|GetFootBoneName) (+ StepStartTime 0.05))))))
  (LocalVariables|SetStartBallHeight (Math|Float|Min(Float) (.z (.Location (CallFunction|GetBonePoseHelperTime _anim_sequence (LocalVariables|GetBallBoneName) StepStartTime))) (.z (.Location (CallFunction|GetBonePoseHelperTime _anim_sequence (LocalVariables|GetBallBoneName) (+ StepStartTime 0.05))))))
  (bind _output_get (LocalVariables|SetStartFrame (Class|AnimationBlueprintLibrary|GetFrameatTime (Variables|Default|GetAnim%20Sequence) StepStartTime)))
  (bind _index (Utilities|FlowControl|ForLoopwithBreak (+ _output_get 1) (Class|AnimationBlueprintLibrary|GetNumFrames (Variables|Default|GetAnim%20Sequence)) :!label _label)
    (:LoopBody
      (LocalVariables|SetCurrentFrame _index)
      (LocalVariables|SetStartFootHeight (Math|Float|Min(Float) (.z (.Location (CallFunction|GetBonePoseHelper (Variables|Default|GetAnim%20Sequence) (LocalVariables|GetFootBoneName) (LocalVariables|GetCurrentFrame)))) (LocalVariables|GetStartFootHeight)))
      (LocalVariables|SetStartBallHeight 0.0)
      (bind _output_get_2 (LocalVariables|SetFootLiftFound (and (> (- (.z (.Location (CallFunction|GetBonePoseHelper (Variables|Default|GetAnim%20Sequence) (LocalVariables|GetFootBoneName) (LocalVariables|GetCurrentFrame)))) (LocalVariables|GetStartFootHeight)) (Variables|Default|GetFootLiftDeltaHeightThreshold)) (> (- (.z (.Location (CallFunction|GetBonePoseHelper (Variables|Default|GetAnim%20Sequence) (LocalVariables|GetBallBoneName) (LocalVariables|GetCurrentFrame)))) (LocalVariables|GetStartBallHeight)) (Variables|Default|GetBallLiftDeltaHeightThreshold)))))
      (if _output_get_2
        (goto _label Break)))
    (:Completed
      (return (Class|AnimationBlueprintLibrary|GetTimeatFrame (Variables|Default|GetAnim%20Sequence) (Math|Integer|Clamp(Integer) (LocalVariables|GetCurrentFrame) 0 (Class|AnimationBlueprintLibrary|GetNumFrames (Variables|Default|GetAnim%20Sequence)))) (LocalVariables|GetFootLiftFound)))))

(fn GetBonePoseHelper
  (params (AnimSequence :type Anim%20Sequence%20Base%20Object%20Reference) (BoneName :type Name) (Frame :type Integer))
  (bind _pose (Class|AnimPoseExtensions|GetAnimPoseatFrame AnimSequence Frame (Utilities|Struct|MakeAnimPoseEvaluationOptions "Raw")))
  (return (.location (Class|AnimPoseExtensions|GetBonePose _pose BoneName "World")) (.rotation (Class|AnimPoseExtensions|GetBonePose _pose BoneName "World"))))

(fn GetBonePoseHelperTime
  (params (AnimSequence :type Anim%20Sequence%20Base%20Object%20Reference) (BoneName :type Name) (Time :type Float%20%28double-precision%29))
  (bind _pose (Class|AnimPoseExtensions|GetAnimPoseatTime AnimSequence Time (Utilities|Struct|MakeAnimPoseEvaluationOptions "Raw")))
  (return (.location (Class|AnimPoseExtensions|GetBonePose _pose BoneName "World")) (.rotation (Class|AnimPoseExtensions|GetBonePose _pose BoneName "World"))))

(fn SetNotifyParams
  (params (Anim%20Notify :type Anim%20Notify%20Object%20Reference) (Is%20Left%20Foot :type Boolean))
  (bind _asanim_notify_footstep (Utilities|Casting|CastToAnimNotify_Footstep Anim%20Notify))
  (Variables|/Game/LocoMotionMatching/Blueprints/AnimNotify/Footsteps/AnimNotify_Footstep.AnimNotify_Footstep_C|SetFootstep%20Type _asanim_notify_footstep (Variables|Default|GetFootstepType))
  (Variables|/Game/LocoMotionMatching/Blueprints/AnimNotify/Footsteps/AnimNotify_Footstep.AnimNotify_Footstep_C|SetLeft%20Foot _asanim_notify_footstep Is%20Left%20Foot))

(fn InitCurveKeys
  (params (CurveName :type Name) (IsLeft :type Boolean))
  (bind (_endtime _footlifted) (CallFunction|GetFootstepEnd 0.0 IsLeft))
  (if (CallFunction|IsFootStartingDown IsLeft)
    (LocalVariables|SetEnd%20Time _endtime)
    (CallFunction|AddKey CurveName 0.0 (Variables|Default|GetPlantHeightValue))
    (if _footlifted
      (CallFunction|AddFootstepEndKeys CurveName (LocalVariables|GetEnd%20Time)))
    (else
      (CallFunction|AddKey CurveName 0.0 (Variables|Default|GetRegularSpeed)))))

(fn IsFootStartingDown
  (params (Is%20Left :type Boolean))
  (Variables|Default|SetFootBoneName (select Is%20Left "foot_l" "foot_r"))
  (Variables|Default|SetBallBoneName (select Is%20Left "ball_l" "ball_r"))
  (return (and (< (.z (.Location (CallFunction|GetBonePoseHelperTime (Variables|Default|GetAnim%20Sequence) (Variables|Default|GetFootBoneName) 0.0))) (Variables|Default|GetStartFootLockThreshold)) (< (.z (.Location (CallFunction|GetBonePoseHelperTime (Variables|Default|GetAnim%20Sequence) (Variables|Default|GetBallBoneName) 0.0))) (Variables|Default|GetStartBallLockThreshold)))))

(fn AddFootstepEndKeys
  (params (Curve :type Name) (Footsep%20End%20Time :type Float%20%28double-precision%29))
  (CallFunction|AddKey Curve Footsep%20End%20Time (Variables|Default|GetPlantHeightValue))
  (if (< (Class|AnimationBlueprintLibrary|GetFrameatTime (Variables|Default|GetAnim%20Sequence) Footsep%20End%20Time) (- (Class|AnimationBlueprintLibrary|GetNumFrames (Variables|Default|GetAnim%20Sequence)) 1))
    (CallFunction|AddKey Curve (Class|AnimationBlueprintLibrary|GetTimeatFrame (Variables|Default|GetAnim%20Sequence) (+ (Class|AnimationBlueprintLibrary|GetFrameatTime (Variables|Default|GetAnim%20Sequence) Footsep%20End%20Time) 1)) (Variables|Default|GetRegularSpeed))))

(fn AddKey
  (params (Curve :type Name) (Time :type Float%20%28double-precision%29) (Value :type Float%20%28double-precision%29))
  (bind _output_get (LocalVariables|SetNewTime (Math|Float|Max(Float) (Variables|Default|GetEarliest%20Safe%20Time) Time)))
  (Class|AnimationBlueprintLibrary|AddFloatCurveKey (Variables|Default|GetAnim%20Sequence) Curve _output_get Value)
  (Variables|Default|SetEarliest%20Safe%20Time (Class|AnimationBlueprintLibrary|GetTimeatFrame (Variables|Default|GetAnim%20Sequence) (+ (Class|AnimationBlueprintLibrary|GetFrameatTime (Variables|Default|GetAnim%20Sequence) (LocalVariables|GetNewTime)) 1)))
  (return))