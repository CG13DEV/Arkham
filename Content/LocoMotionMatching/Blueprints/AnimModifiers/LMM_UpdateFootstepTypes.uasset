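; LMM_UpdateFootstepTypes is an animation modifier that bulk-updates the footstep type on an animation sequence's existing footstep notifies.
; On apply, it reads the notify events from the left and right FootLock notify tracks.
; Each event that casts to AnimNotify_Footstep has its FootstepType overwritten with the modifier's NewFootstepType value.
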(event EventOnApply
  (params (AnimationSequence :type Anim%20Sequence%20Object%20Reference))
  (Variables|Default|SetAnim%20Sequence AnimationSequence)
  (CallFunction|ProcessNotifies (Class|AnimationBlueprintLibrary|GetAnimationNotifyEventsforTrack (Variables|Default|GetAnim%20Sequence) "FootLock_L_Notifs"))
  (CallFunction|ProcessNotifies (Class|AnimationBlueprintLibrary|GetAnimationNotifyEventsforTrack (Variables|Default|GetAnim%20Sequence) "FootLock_R_Notifs")))

(fn ProcessNotifies
  (params (Notifies :type Array%20of%20Anim%20Notify%20Event%20Structures))
  (for _array_element Notifies
    (bind _asanim_notify_footstep (Utilities|Casting|CastToAnimNotify_Footstep (.Notify (Utilities|Struct|BreakAnimNotifyEvent _array_element))))
    (Variables|/Game/LocoMotionMatching/Blueprints/AnimNotify/Footsteps/AnimNotify_Footstep.AnimNotify_Footstep_C|SetFootstep%20Type _asanim_notify_footstep (Variables|Default|GetNew%20Footstep%20Type))))